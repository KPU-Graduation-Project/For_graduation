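; BP_Larva is a suicide-bomber enemy that moves toward the player and, on arrival, plays a ready sound and sets an Explosion flag.
; Event_Explosion, not called in this graph, destroys it with effects and sends AttackMessage to unique pawns found by a sphere trace.
; Overlaps destroy the other actor; cannonball hits are counted, and past five they reveal extra meshes and let a match bullet burst the larva.
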(event `self.ReceiveBeginPlay`
  (`|AIMoveTo` self (0.0 0.0 0.0) (`GameplayStatics.GetPlayerPawn` 0) 300.0
    (:`OnSuccess`
      (`GameplayStatics.PlaySoundAtLocation` "/Game/Asset/Music/Monster/Larva/Larva_Ready.Larva_Ready" (`self.K2_GetActorLocation`) (struct) 1.0 1.0 0.0 null null null)
      (`KismetSystemLibrary.Delay` 0.5)
      (set `self.Explosion` true))))

(event `self.ReceiveActorBeginOverlap`
  (params (OtherActor :type "Actor Object Reference"))
  (bind _returnvalue (`self.K2_GetActorLocation`))
  (bind _count (`self.Count`))
  (bind _returnvalue_2 (> _count 5))
  (`self.K2_DestroyActor` OtherActor)
  (cast `/Game/Asset/Actor/Weapon/Cannon/BP_WeaponCannonBall` OtherActor
    (:`then`
      (`/Engine/EditorBlueprintResources/StandardMacros.IncrementInt` _count
        (:`  `
          (if _returnvalue_2
            (`SceneComponent.SetVisibility` (`self.StaticMesh`) true false)
            (`SceneComponent.SetVisibility` (`self.StaticMesh1`) true false)
            (`SceneComponent.SetVisibility` (`self.StaticMesh2`) true false)
            (`SceneComponent.SetVisibility` (`self.StaticMesh3`) true false)
            (`SceneComponent.SetVisibility` (`self.StaticMesh4`) true false)))))
    (:`CastFailed`
      (cast `/Game/Asset/Actor/Weapon/Gun/BP_WeaponMatchBullet` OtherActor)
      (if _returnvalue_2
        (`self.K2_DestroyActor`)
        (`GameplayStatics.PlaySoundAtLocation` "/Game/Asset/Music/Weapon/Explosion/Explosion.Explosion" _returnvalue (struct) 1.0 1.0 0.0 null null null)
        (`GameplayStatics.SpawnEmitterAtLocation` "/Game/Map/Particle/P_Burst.P_Burst" _returnvalue (struct) (0.2 0.2 0.2))
        (`GameplayStatics.SpawnEmitterAtLocation` "/Game/Map/Particle/P_MonExclusion.P_MonExclusion" _returnvalue (struct) (2.0 2.0 2.0))))))

(event `Event_Explosion`
  (bind _returnvalue (`self.K2_GetActorLocation`))
  (bind _x (.x _returnvalue))
  (bind _y (.y _returnvalue))
  (bind _returnvalue_2 (+ (.z _returnvalue) 370.0))
  (bind _output_get (set `self.Explosion_Point` (`KismetMathLibrary.MakeVector` _x _y _returnvalue_2)))
  (`self.K2_DestroyActor`)
  (`GameplayStatics.PlaySoundAtLocation` "/Game/Asset/Music/Monster/Larva/Larva_Attack.Larva_Attack" _output_get (struct) 1.0 1.0 0.0 null null null)
  (`GameplayStatics.SpawnEmitterAtLocation` "/Game/Map/Particle/P_MonExclusion.P_MonExclusion" (`KismetMathLibrary.MakeVector` _x _y _returnvalue_2) (struct) (8.0 8.0 8.0))
  (bind _outhits (`KismetSystemLibrary.SphereTraceMultiByProfile` _output_get _returnvalue 300.0 "OnlyPawn"))
  (for _array_element _outhits
    (`KismetArrayLibrary.Array_AddUnique` (`self.HitActor`) (`.HitActor` (`GameplayStatics.BreakHitResult` _array_element))))
  (for _array_element_2 (`self.HitActor`)
    (message `/Game/Asset/Component/Damage.Attack` _array_element_2)))

(fn `UserConstructionScript`)