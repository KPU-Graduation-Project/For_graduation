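; BP_Target is a rotatable object with a selectable mesh that turns when triggered and drives a linked actor by its angle.
; Four Front and four Back overlap triggers send forward or backward spin requests to NetworkModule, while SetRotation separately offsets the target yaw.
; Tick eases toward that rotation, counts yaw wraparounds and passes the cumulative multi-turn angle to the actor assigned through SetChild.
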(event `self.ReceiveBeginPlay`
  (bind (_returnvalue_roll _returnvalue_pitch _returnvalue_yaw) (`KismetMathLibrary.BreakRotator` (`SceneComponent.K2_GetComponentRotation` (`self.Target`))))
  (set `self.Angle` (`KismetMathLibrary.ClampAxis` _returnvalue_yaw))
  (set `self.targetRotation` (`KismetMathLibrary.MakeRotator` _returnvalue_roll _returnvalue_pitch _returnvalue_yaw)))

(event `self.ReceiveTick`
  (params (DeltaSeconds :type "Float (single-precision)"))
  (`self.K2_SetActorRotation` (`KismetMathLibrary.RInterpTo` (`self.K2_GetActorRotation`) (`self.targetRotation`) DeltaSeconds 3.0))
  (`self.SetSpinAngle`)
  (message `/Game/Asset/Component/ObjectConnection.ChangeAngle` (`self.Actor`) (+ (* (`self.SpinCount`) 360.0) (`self.Angle`))))

(event `self.Front1.OnComponentBeginOverlap`
  (params (OverlappedComponent :type "PrimitiveComponent Object Reference") (OtherActor :type "Actor Object Reference") (OtherComp :type "PrimitiveComponent Object Reference") (OtherBodyIndex :type Integer) (bFromSweep :type Boolean) (SweepResult :type "HitResult Structure (by ref)"))
  (`NetworkModule.TargetSpin` (`self.NetworkModule`) self true :!label _label))

(event `self.Back1.OnComponentBeginOverlap`
  (params (OverlappedComponent :type "PrimitiveComponent Object Reference") (OtherActor :type "Actor Object Reference") (OtherComp :type "PrimitiveComponent Object Reference") (OtherBodyIndex :type Integer) (bFromSweep :type Boolean) (SweepResult :type "HitResult Structure (by ref)"))
  (`NetworkModule.TargetSpin` (`self.NetworkModule`) self false :!label _label_2))

(event `self.Front2.OnComponentBeginOverlap`
  (params (OverlappedComponent :type "PrimitiveComponent Object Reference") (OtherActor :type "Actor Object Reference") (OtherComp :type "PrimitiveComponent Object Reference") (OtherBodyIndex :type Integer) (bFromSweep :type Boolean) (SweepResult :type "HitResult Structure (by ref)"))
  (goto _label))

(event `self.Back2.OnComponentBeginOverlap`
  (params (OverlappedComponent :type "PrimitiveComponent Object Reference") (OtherActor :type "Actor Object Reference") (OtherComp :type "PrimitiveComponent Object Reference") (OtherBodyIndex :type Integer) (bFromSweep :type Boolean) (SweepResult :type "HitResult Structure (by ref)"))
  (goto _label_2))

(event `self.Front3.OnComponentBeginOverlap`
  (params (OverlappedComponent :type "PrimitiveComponent Object Reference") (OtherActor :type "Actor Object Reference") (OtherComp :type "PrimitiveComponent Object Reference") (OtherBodyIndex :type Integer) (bFromSweep :type Boolean) (SweepResult :type "HitResult Structure (by ref)"))
  (goto _label))

(event `self.Back3.OnComponentBeginOverlap`
  (params (OverlappedComponent :type "PrimitiveComponent Object Reference") (OtherActor :type "Actor Object Reference") (OtherComp :type "PrimitiveComponent Object Reference") (OtherBodyIndex :type Integer) (bFromSweep :type Boolean) (SweepResult :type "HitResult Structure (by ref)"))
  (goto _label_2))

(event `self.Front4.OnComponentBeginOverlap`
  (params (OverlappedComponent :type "PrimitiveComponent Object Reference") (OtherActor :type "Actor Object Reference") (OtherComp :type "PrimitiveComponent Object Reference") (OtherBodyIndex :type Integer) (bFromSweep :type Boolean) (SweepResult :type "HitResult Structure (by ref)"))
  (goto _label))

(event `self.Back4.OnComponentBeginOverlap`
  (params (OverlappedComponent :type "PrimitiveComponent Object Reference") (OtherActor :type "Actor Object Reference") (OtherComp :type "PrimitiveComponent Object Reference") (OtherBodyIndex :type Integer) (bFromSweep :type Boolean) (SweepResult :type "HitResult Structure (by ref)"))
  (goto _label_2))

(fn `SetChild`
  (params (Child :type "Actor Object Reference"))
  (set `self.Actor` Child))

(fn `SetMesh`
  (params (`Mesh ID` :type Integer))
  (`StaticMeshComponent.SetStaticMesh` (`self.Target`) (`|GetArrayItem` (`self.Mesh List`) `Mesh ID`))
  (set `self.Mesh ID` `Mesh ID`))

(fn `SetRotation`
  (params (Direction :type "Float (double-precision)"))
  (bind (_targetrotation_roll _targetrotation_pitch _targetrotation_yaw) (`KismetMathLibrary.BreakRotator` (`self.targetRotation`)))
  (set `self.targetRotation` (`KismetMathLibrary.MakeRotator` 0.0 0.0 (+ Direction _targetrotation_yaw))))

(fn `SetSpinAngle`
  (locals (CurrentAngle :type "Float (double-precision)"))
  (bind (_returnvalue_roll _returnvalue_pitch _returnvalue_yaw) (`KismetMathLibrary.BreakRotator` (`self.K2_GetActorRotation`)))
  (bind _returnvalue (`KismetMathLibrary.ClampAxis` (`self.Angle`)))
  (bind _output_get (set `local.CurrentAngle` (`KismetMathLibrary.ClampAxis` _returnvalue_yaw)))
  (if (== _output_get _returnvalue)
    _
    (elif (> (`KismetMathLibrary.Abs` (- _output_get _returnvalue)) 270.0)
      (if (< (`self.Angle`) (`local.CurrentAngle`))
        (set `self.SpinCount` (- (`self.SpinCount`) 1))
        (else
          (set `self.SpinCount` (+ (`self.SpinCount`) 1))))
      (set `self.Angle` (`local.CurrentAngle`))
      (else
        (set `self.Angle` (`local.CurrentAngle`))))))

(fn `UserConstructionScript`
  (`StaticMeshComponent.SetStaticMesh` (`self.Target`) (`|GetArrayItem` (`self.Mesh List`) (`self.Mesh ID`))))