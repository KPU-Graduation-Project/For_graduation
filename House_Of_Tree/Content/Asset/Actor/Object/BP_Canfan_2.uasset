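; BP_Canfan_2 is a networked physics object that rotates when any of its four hit components (R, L, U, D) is struck.
; A hit raises or lowers the target Angle in fixed steps, depending on the struck component's world roll.
; Once ownership is set, by the VR player controller's DESETOWNER dispatcher or SetOwned, Tick eases roll toward Angle and passes the actor to NetworkModule.ObjectData.
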(event `self.ReceiveBeginPlay`
  (bind _asbp_vrplayer_controller (cast `/Game/Asset/Component/BP_VRPlayerController` (`GameplayStatics.GetPlayerController` 0)))
  (add `VRPlayerController_Base.DE_SETOWNER` _asbp_vrplayer_controller (delegate `DE_SETOWNER_Event_0`)))

(event `DE_SETOWNER_Event_0`
  (set `self.Owned` true))

(event `self.ReceiveTick`
  (params (DeltaSeconds :type "Float (single-precision)"))
  (if (`self.Owned`)
    (`self.K2_SetActorRotation` (`KismetMathLibrary.RInterpTo` (`self.K2_GetActorRotation`) (`KismetMathLibrary.MakeRotator` (`self.Angle`) 0.0 -90.0) DeltaSeconds 0.5))
    (`NetworkModule.ObjectData` (`self.NetworkModule`) self)))

(event `self.R.OnComponentHit`
  (params (HitComponent :type "PrimitiveComponent Object Reference") (OtherActor :type "Actor Object Reference") (OtherComp :type "PrimitiveComponent Object Reference") (NormalImpulse :type "Vector Structure") (Hit :type "HitResult Structure (by ref)"))
  (`self.Set Angle` (`self.R`)))

(event `self.L.OnComponentHit`
  (params (HitComponent :type "PrimitiveComponent Object Reference") (OtherActor :type "Actor Object Reference") (OtherComp :type "PrimitiveComponent Object Reference") (NormalImpulse :type "Vector Structure") (Hit :type "HitResult Structure (by ref)"))
  (`self.Set Angle` (`self.L`)))

(event `self.U.OnComponentHit`
  (params (HitComponent :type "PrimitiveComponent Object Reference") (OtherActor :type "Actor Object Reference") (OtherComp :type "PrimitiveComponent Object Reference") (NormalImpulse :type "Vector Structure") (Hit :type "HitResult Structure (by ref)"))
  (`self.Set Angle` (`self.U`)))

(event `self.D.OnComponentHit`
  (params (HitComponent :type "PrimitiveComponent Object Reference") (OtherActor :type "Actor Object Reference") (OtherComp :type "PrimitiveComponent Object Reference") (NormalImpulse :type "Vector Structure") (Hit :type "HitResult Structure (by ref)"))
  (`self.Set Angle` (`self.D`)))

(fn `Set Angle`
  (params (Target :type "SceneComponent Object Reference"))
  (bind _returnvalue_roll (`KismetMathLibrary.BreakRotator` (`SceneComponent.K2_GetComponentRotation` Target)))
  (bind _returnvalue (`KismetMathLibrary.ClampAxis` _returnvalue_roll))
  (if (`self.Owned`)
    (if (or (`KismetMathLibrary.InRange_FloatFloat` _returnvalue 271.0 360.0 false) (`KismetMathLibrary.InRange_FloatFloat` _returnvalue 0.0 89.0 true false))
      (set `self.Angle` (+ (`self.Angle`) 10.0))
      (elif (`KismetMathLibrary.InRange_FloatFloat` _returnvalue 91.0 269.0 false false)
        (set `self.Angle` (- (`self.Angle`) 10.0))))))

(fn `SetOwned`
  (bind _output_get (set `self.owned` true))
  (`PrimitiveComponent.SetSimulatePhysics` (`self.StaticMesh`) _output_get))

(fn `TestFunc`
  (`KismetSystemLibrary.PrintString` "Sucess"))

(fn `UserConstructionScript`)