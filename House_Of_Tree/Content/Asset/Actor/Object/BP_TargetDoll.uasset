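; BP_TargetDoll is a target doll actor whose static mesh is selected from a list by an index.
; The construction script applies the MeshList entry at MeshID to the TargetDoll component.
; SetMesh lets callers switch to another entry and stores the new index in MeshID.
; The event graph holds only empty placeholder events, so the actor has no gameplay logic of its own.
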(fn `SetMesh`
  (params (`Mesh ID` :type Integer))
  (`StaticMeshComponent.SetStaticMesh` (`self.TargetDoll`) (`|GetArrayItem` (`self.Mesh List`) `Mesh ID`))
  (set `self.Mesh ID` `Mesh ID`))

(fn `UserConstructionScript`
  (`StaticMeshComponent.SetStaticMesh` (`self.TargetDoll`) (`|GetArrayItem` (`self.Mesh List`) (`self.Mesh ID`))))