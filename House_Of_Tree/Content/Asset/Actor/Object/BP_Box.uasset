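; BP_Box is a box object actor that stays static until more than 30 actors are attached to it, then simulates physics.
; Its mesh comes from MeshList by MeshID, set in the construction script or through SetMesh.
; Tick prints the attached actor count and uses a DoOnce to switch on physics past that threshold.
; SetChild only stores an actor reference.
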(event `self.ReceiveBeginPlay`
  (`PrimitiveComponent.SetSimulatePhysics` (`self.Mesh`) false))

(event `self.ReceiveTick`
  (params (DeltaSeconds :type "Float (single-precision)"))
  (bind _returnvalue (`KismetArrayLibrary.Array_Length` (`self.GetAttachedActors` true)))
  (`KismetSystemLibrary.PrintString` (`KismetStringLibrary.Conv_IntToString` _returnvalue))
  (if (> _returnvalue 30)
    (`/Engine/EditorBlueprintResources/StandardMacros.DoOnce` false
      (:`Completed`
        (`PrimitiveComponent.SetSimulatePhysics` (`self.Mesh`) true)))))

(fn `SetChild`
  (params (Actor :type "Actor Object Reference"))
  (set `self.Actor` Actor))

(fn `SetMesh`
  (params (`Mesh ID` :type Integer))
  (`StaticMeshComponent.SetStaticMesh` (`self.Mesh`) (`|GetArrayItem` (`self.Mesh List`) `Mesh ID`))
  (set `self.Mesh ID` `Mesh ID`))

(fn `UserConstructionScript`
  (`StaticMeshComponent.SetStaticMesh` (`self.Mesh`) (`|GetArrayItem` (`self.Mesh List`) (`self.Mesh ID`))))