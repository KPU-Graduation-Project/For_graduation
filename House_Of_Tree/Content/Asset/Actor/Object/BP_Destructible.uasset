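; BP_Destructible is a destructible object that breaks apart with a barricade explosion sound when it takes any damage.
; On damage it disables the Box collision, applies radius damage to its own destructible Mesh at the actor location to fracture it, and plays the sound.
; The construction script picks the mesh from MeshList by MeshID, and SetMesh swaps the mesh and stores the new ID.
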(event `self.ReceiveAnyDamage`
  (params (Damage :type "Float (single-precision)") (DamageType :type "DamageType Object Reference") (InstigatedBy :type "Controller Object Reference") (DamageCauser :type "Actor Object Reference"))
  (bind _returnvalue (`self.K2_GetActorLocation`))
  (`PrimitiveComponent.SetCollisionProfileName` (`self.Box`) "NoCollision" true)
  (`DestructibleComponent.ApplyRadiusDamage` (`self.Mesh`) 10.0 _returnvalue 200.0 0.0 true)
  (`GameplayStatics.PlaySoundAtLocation` "/Game/Asset/Music/Weapon/Explosion/Explosion_Barricade.Explosion_Barricade" _returnvalue (struct) 1.0 1.0 0.0 null null null))

(fn `SetMesh`
  (params (`Mesh ID` :type Integer))
  (`DestructibleComponent.SetDestructibleMesh` (`self.Mesh`) (`|GetArrayItem` (`self.Mesh List`) `Mesh ID`))
  (set `self.Mesh ID` `Mesh ID`))

(fn `UserConstructionScript`
  (`DestructibleComponent.SetDestructibleMesh` (`self.Mesh`) (`|GetArrayItem` (`self.Mesh List`) (`self.Mesh ID`))))