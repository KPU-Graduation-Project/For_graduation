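; VR boy player character with a weapon whose shots are sent to the server.
; It uses eye-level tracking and, on Tick for the first local player only, turns the mesh to the HMD yaw and updates Speed for animation.
; Right trigger press and release both drive one FlipFlop that sets Shoot.
; While Shoot is set, Tick polls BPWeaponBoy and forwards successful shots' location and rotation through NetworkModule.
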(event `self.ReceiveBeginPlay`
  ;[1 1 1] 카메라 위치로 HMD 높이 지정
  (`HeadMountedDisplayFunctionLibrary.SetTrackingOrigin` "Eye"))

(event `self.ReceiveTick`
  (params (DeltaSeconds :type "Float (single-precision)"))
  (if (== (`GameplayStatics.GetPlayerCharacter` 0) self)
    ;[1 1 1] 캐릭터 회전 설정
    (`SceneComponent.K2_SetWorldRotation` (`self.Mesh`) (`KismetMathLibrary.MakeRotator` 0.0 0.0 (+ (.yaw (`HeadMountedDisplayFunctionLibrary.GetOrientationAndPosition`)) 180.0)) false false)
    ;[1 1 1] 애니메이션을 위한 Speed
    (set `self.Speed` (`KismetMathLibrary.VSize` (`self.GetVelocity`)))
    ;[1 0.4167 0.4482] 발사 명령을 서버에 전송
    (if (`self.Shoot`)
      (bind (_shoot _location _rotation) (`/Game/Asset/Actor/Weapon/BP_WeaponBoy.Shoot Weapon` (`self.BP_WeaponBoy`)))
      (if _shoot
        (`NetworkModule.ShootBullet` (`self.NetworkModule`) _location _rotation)))))

(event `InputAction|TriggerRight`
  (params (Key :type "Key Structure"))
  ;[1 1 1] 토글 방식으로 발사
  (:`Pressed`
    (bind _isa (`/Engine/EditorBlueprintResources/StandardMacros.FlipFlop` :!label _label)
      (:`A`
        _)
      (:`B`
        _))
    (set `self.Shoot` _isa))
  (:`Released`
    (goto _label)))

(fn `UserConstructionScript`)