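; BP_WeaponBoy is a weapon Blueprint that fires BP_WeaponMatchBullet projectiles from its Muzzle socket.
; ShootWeapon spawns a bullet at the socket's world transform, passes on the weapon's owner, and fires it along the socket's forward vector.
; A ShootGap timer, reset to TimeGap per shot and counted down on Tick, limits fire rate.
; A helper returns any socket's location in parent bone space.
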(event `self.ReceiveBeginPlay`
  (set `self.ShootGap` 0.0))

(event `self.ReceiveTick`
  (params (DeltaSeconds :type "Float (single-precision)"))
  (bind _shootgap (`self.ShootGap`))
  (if (> _shootgap 0.0)
    (set `self.ShootGap` (- _shootgap DeltaSeconds))))

(fn `Get Socket Position`
  (params (`Socket Name` :type Name))
  (returns (`Socket Position` :type "Vector Structure"))
  (bind _returnvalue_location (`KismetMathLibrary.BreakTransform` (`self.GetSocketTransform` `Socket Name` "RTS_ParentBoneSpace")))
  (return _returnvalue_location))

(fn `Shoot Weapon`
  (bind (_returnvalue_location _returnvalue_rotation) (`KismetMathLibrary.BreakTransform` (`self.GetSocketTransform` "Muzzle")))
  (if (<= (`self.ShootGap`) 0.0)
    (bind _returnvalue (`|SpawnActorFromClass` "/Game/Asset/Actor/Weapon/Gun/BP_WeaponMatchBullet.BP_WeaponMatchBullet_C" (`KismetMathLibrary.MakeTransform` _returnvalue_location _returnvalue_rotation) "Undefined" "OverrideRootScale" (`self.GetOwner`) null))
    (`WeaponMatchBullet.FireInDirection` _returnvalue (`KismetMathLibrary.Conv_RotatorToVector` _returnvalue_rotation))
    (set `self.ShootGap` (`self.TimeGap`))))