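; BP_Larva_2 is a suicide-bomber larva enemy that chases the first pawn detected nearby.
; On arrival or via CallExplosion it sets an Explosion flag after a short delay; Event_Explosion destroys it and sends AttackMessage to pawns caught in a sphere trace.
; Repeated cannonball hits reveal extra meshes and slow it, after which a match bullet destroys it without area damage.
; SendPacket reports non-idle State to NetworkModule at a throttled rate.
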(event `self.ReceiveBeginPlay`)

(event `self.ReceiveTick`
  (params (DeltaSeconds :type "Float (single-precision)"))
  (bind _returnvalue (`self.K2_GetActorLocation`))
  (`/Engine/EditorBlueprintResources/StandardMacros.DoOnce` false :!label _label
    (:`Completed`
      (bind (_outhit _returnvalue_2) (`KismetSystemLibrary.SphereTraceSingleByProfile` _returnvalue _returnvalue 1200.0 "OnlyPawn"))
      (if _returnvalue_2
        (set `self.State` 1)
        (`|AIMoveTo` self (0.0 0.0 0.0) (`.HitActor` (`GameplayStatics.BreakHitResult` _outhit)) 300.0
          (:`OnSuccess`
            (set `self.State` 2)
            (`GameplayStatics.PlaySoundAtLocation` "/Game/Asset/Music/Monster/Larva/Larva_Ready.Larva_Ready" (`self.K2_GetActorLocation`) (struct) 1.0 1.0 0.0 null null null)
            (`KismetSystemLibrary.Delay` 0.5)
            (set `self.Explosion` true)))
        (else
          (goto _label :!via `Reset`))))))

(event `self.ReceiveActorBeginOverlap`
  (params (OtherActor :type "Actor Object Reference"))
  (bind _returnvalue (`self.K2_GetActorLocation`))
  (bind _count (`self.Count`))
  (bind _returnvalue_2 (> _count 3))
  (cast `/Game/Asset/Actor/Weapon/Cannon/BP_WeaponCannonBall` OtherActor
    (:`then`
      (`/Engine/EditorBlueprintResources/StandardMacros.IncrementInt` _count
        (:`  `
          (if _returnvalue_2
            (`SceneComponent.SetVisibility` (`self.StaticMesh`) true false)
            (`SceneComponent.SetVisibility` (`self.StaticMesh1`) true false)
            (`SceneComponent.SetVisibility` (`self.StaticMesh2`) true false)
            (`SceneComponent.SetVisibility` (`self.StaticMesh3`) true false)
            (`SceneComponent.SetVisibility` (`self.StaticMesh4`) true false)
            (set `CharacterMovementComponent.MaxWalkSpeed` 20.0 (`self.CharacterMovement`))
            (`GameplayStatics.PlaySoundAtLocation` "/Game/Asset/Music/Monster/Larva/Larva_Sapped.Larva_Sapped" (`self.K2_GetActorLocation`) (struct) 1.0 1.0 0.0 null null null)))))
    (:`CastFailed`
      (cast `/Game/Asset/Actor/Weapon/Gun/BP_WeaponMatchBullet` OtherActor)
      (if _returnvalue_2
        (`self.K2_DestroyActor`)
        (`GameplayStatics.PlaySoundAtLocation` "/Game/Asset/Music/Weapon/Explosion/Explosion.Explosion" _returnvalue (struct) 1.0 1.0 0.0 null null null)
        (`GameplayStatics.SpawnEmitterAtLocation` "/Game/Map/Particle/P_Burst.P_Burst" _returnvalue (struct) (0.2 0.2 0.2))
        (`GameplayStatics.SpawnEmitterAtLocation` "/Game/Map/Particle/P_MonExclusion.P_MonExclusion" _returnvalue (struct) (2.0 2.0 2.0))))))

(event `Event_Explosion`
  (bind _returnvalue (`self.K2_GetActorLocation`))
  (bind _x (.x _returnvalue))
  (bind _y (.y _returnvalue))
  (bind _returnvalue_2 (+ (.z _returnvalue) 370.0))
  (bind _output_get (set `self.Explosion_Point` (`KismetMathLibrary.MakeVector` _x _y _returnvalue_2)))
  (`self.K2_DestroyActor`)
  (`GameplayStatics.PlaySoundAtLocation` "/Game/Asset/Music/Monster/Larva/Larva_Attack.Larva_Attack" _output_get (struct) 1.0 1.0 0.0 null null null)
  (`GameplayStatics.SpawnEmitterAtLocation` "/Game/Map/Particle/P_MonExclusion.P_MonExclusion" (`KismetMathLibrary.MakeVector` _x _y _returnvalue_2) (struct) (8.0 8.0 8.0))
  (bind _outhits (`KismetSystemLibrary.SphereTraceMultiByProfile` _output_get _returnvalue 300.0 "OnlyPawn"))
  (for _array_element _outhits
    (`KismetArrayLibrary.Array_AddUnique` (`self.Hit actor`) (`.HitActor` (`GameplayStatics.BreakHitResult` _array_element))))
  (for _array_element_2 (`self.Hit actor`)
    (message `/Game/Asset/Component/Damage.Attack` _array_element_2)))

(event `Call Explosion`
  (`GameplayStatics.PlaySoundAtLocation` "/Game/Asset/Music/Monster/Larva/Larva_Ready.Larva_Ready" (`self.K2_GetActorLocation`) (struct) 1.0 1.0 0.0 null null null)
  (`KismetSystemLibrary.Delay` 0.5)
  (set `self.Explosion` true))

(fn `SendPacket`
  (params (`Deleta Time` :type "Float (double-precision)"))
  (if true
    (if (!= (`self.State`) 0)
      (if (< (`self.RemainTime`) 0.0)
        (`NetworkModule.Monster` (`self.NetworkModule`) self (`self.State`))
        (set `self.RemainTime` (`self.SendRate`))
        (else
          (set `self.RemainTime` (- (`self.RemainTime`) `Deleta Time`))))))
  (return))

(fn `UserConstructionScript`)