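; Lobby UI actor that hosts a widget component and relays VR player controller events to the lobby and room screens.
; On BeginPlay it caches LobbyUI and RoomUI, sets itself as their parent, and binds to controller dispatchers.
; ID, room entry and exit, and user state changes are forwarded to the child widgets.
; The local player entering a room switches the display to RoomUI, and RoomOut switches it back to LobbyUI.
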(event `self.ReceiveActorBeginOverlap`
  (params (OtherActor :type "Actor Object Reference")))

(event `self.ReceiveTick`
  (params (DeltaSeconds :type "Float (single-precision)")))

(event `self.ReceiveBeginPlay`
  (bind _aswidget_ui (cast `/Game/Asset/Lobby/UI/WidgetUI` (`WidgetComponent.GetWidget` (`self.UI`))))
  (bind _output_get (set `self.LobbyUI` (`/Game/Asset/Lobby/UI/WidgetUI.LobbyUI` _aswidget_ui)))
  (`/Game/Asset/Lobby/UI/LobbyUI.SetParent` _output_get self)
  (bind _output_get_2 (set `self.RoomUI` (`/Game/Asset/Lobby/UI/WidgetUI.RoomUI` _aswidget_ui)))
  (`/Game/Asset/Lobby/UI/RoomUI.Set Parent` _output_get_2 self)
  (bind _asbp_vrplayer_controller (cast `/Game/Asset/Component/BP_VRPlayerController` (`GameplayStatics.GetPlayerController` 0)))
  (add `VRPlayerController_Base.DE_SetID` _asbp_vrplayer_controller (delegate `SetID`))
  (add `VRPlayerController_Base.DE_PlayerEnterRoom` _asbp_vrplayer_controller (delegate `PlayerEnterRoom`))
  (add `VRPlayerController_Base.DE_UserEnterRoom` _asbp_vrplayer_controller (delegate `UserEnterRoom`))
  (add `VRPlayerController_Base.DE_ExitRoom` _asbp_vrplayer_controller (delegate `Exit Room`))
  (add `VRPlayerController_Base.DE_ChangeState` _asbp_vrplayer_controller (delegate `Change User State`)))

(event `Exit Room`
  (params (ID3 :type Integer))
  (bind _roomui (`self.RoomUI`))
  (`KismetSystemLibrary.PrintString` "Exit Room")
  (`/Engine/EditorBlueprintResources/StandardMacros.IsValid` _roomui
    (:`Is Valid`
      (`/Game/Asset/Lobby/UI/RoomUI.Exit User` _roomui ID3))))

(event `Change User State`
  (params (ID1 :type Integer) (roomMaster :type Boolean) (Character :type Integer) (isReady :type Boolean))
  (bind _roomui (`self.RoomUI`))
  (`KismetSystemLibrary.PrintString` "Change User State")
  (`/Engine/EditorBlueprintResources/StandardMacros.IsValid` _roomui
    (:`Is Valid`
      (`/Game/Asset/Lobby/UI/RoomUI.Change User State` _roomui ID1 roomMaster Character isReady))))

(event `SetID`
  (params (ID3 :type Integer))
  (bind _lobbyui (`self.LobbyUI`))
  (bind _roomui (`self.RoomUI`))
  (`/Engine/EditorBlueprintResources/StandardMacros.IsValid` _lobbyui
    (:`Is Valid`
      (`/Game/Asset/Lobby/UI/LobbyUI.Set ID` _lobbyui ID3)
      (`/Engine/EditorBlueprintResources/StandardMacros.IsValid` _roomui
        (:`Is Valid`
          (`/Game/Asset/Lobby/UI/RoomUI.Set ID` _roomui ID3))))))

(event `Room Out`
  (bind _aswidget_ui (cast `/Game/Asset/Lobby/UI/WidgetUI` (`WidgetComponent.GetWidget` (`self.UI`))))
  (`/Game/Asset/Lobby/UI/WidgetUI.Change Widget` _aswidget_ui (`self.LobbyUI`)))

(event `PlayerEnterRoom`
  (params (ID1 :type Integer) (roomMaster :type Boolean) (Character :type Integer) (isReady :type Boolean))
  (bind _roomui (`self.RoomUI`))
  (bind _lobbyui (`self.LobbyUI`))
  (`KismetSystemLibrary.PrintString` "Player Enter Room")
  (`/Engine/EditorBlueprintResources/StandardMacros.IsValid` _lobbyui
    (:`Is Valid`
      (`/Game/Asset/Lobby/UI/LobbyUI.Room In` _lobbyui)
      (`/Engine/EditorBlueprintResources/StandardMacros.IsValid` _roomui
        (:`Is Valid`
          (`/Game/Asset/Lobby/UI/RoomUI.Enter Room` _roomui ID1 roomMaster Character isReady)
          (bind _aswidget_ui (cast `/Game/Asset/Lobby/UI/WidgetUI` (`WidgetComponent.GetWidget` (`self.UI`))))
          (`/Game/Asset/Lobby/UI/WidgetUI.Change Widget` _aswidget_ui _roomui))))))

(event `UserEnterRoom`
  (params (ID1 :type Integer) (roomMaster :type Boolean) (Character :type Integer) (isReady :type Boolean))
  (bind _roomui (`self.RoomUI`))
  (`KismetSystemLibrary.PrintString` "User Enter Room")
  (`/Engine/EditorBlueprintResources/StandardMacros.IsValid` _roomui
    (:`Is Valid`
      (`/Game/Asset/Lobby/UI/RoomUI.Enter User` _roomui ID1 roomMaster Character isReady))))

(fn `UserConstructionScript`)