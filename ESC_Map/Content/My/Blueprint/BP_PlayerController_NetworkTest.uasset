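; BP_PlayerController_NetworkTest is a player controller, named for network testing, that moves and turns its controlled pawn from axis input.
; The MovementAxisRight X and Y axes add movement input along the pawn's right and forward vectors.
; MovementAxisLeft_Y adds scaled yaw input to the controller, with no delta-time factor.
; Each handler first checks for a valid pawn, and no explicit RPC or replication logic is present.
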(event `InputAxis|MovementAxisRight_X`
  (params (AxisValue :type "Float (single-precision)"))
  (bind _returnvalue (`self.K2_GetPawn`))
  (`/Engine/EditorBlueprintResources/StandardMacros.IsValid` _returnvalue
    (:`Is Valid`
      (`Pawn.AddMovementInput` _returnvalue (`self.GetActorRightVector` _returnvalue) AxisValue false))))

(event `InputAxis|MovementAxisRight_Y`
  (params (AxisValue :type "Float (single-precision)"))
  (bind _returnvalue (`self.K2_GetPawn`))
  (`/Engine/EditorBlueprintResources/StandardMacros.IsValid` _returnvalue
    (:`Is Valid`
      (`Pawn.AddMovementInput` _returnvalue (`self.GetActorForwardVector` _returnvalue) AxisValue false))))

(event `InputAxis|MovementAxisLeft_Y`
  (params (AxisValue :type "Float (single-precision)"))
  (`/Engine/EditorBlueprintResources/StandardMacros.IsValid` (`self.K2_GetPawn`)
    (:`Is Valid`
      (`self.AddYawInput` (* AxisValue 10.0)))))

(fn `UserConstructionScript`)