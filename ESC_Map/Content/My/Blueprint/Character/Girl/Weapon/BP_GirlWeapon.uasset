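; Weapon actor for the Girl character that fires BP_MyMatchGun projectiles from its static mesh's Muzzle socket.
; ShootWeapon spawns the projectile with the player pawn as owner and instigator, then launches it along the socket's forward vector.
; A ShootGap cooldown, reset to TimeGap per shot and counted down on Tick, limits the fire rate.
; A helper returns any socket's location in parent bone space.
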(event `self.ReceiveBeginPlay`
  (set `self.ShootGap` 0.0))

(event `self.ReceiveTick`
  (params (DeltaSeconds :type "Float (single-precision)"))
  (bind _shootgap (`self.ShootGap`))
  (if (> _shootgap 0.0)
    (set `self.ShootGap` (- _shootgap DeltaSeconds))))

(fn `Get Scoekt Position`
  (params (`Socket Name` :type Name))
  (returns (`Socket Position` :type "Vector Structure"))
  (bind _returnvalue_location (`KismetMathLibrary.BreakTransform` (`SceneComponent.GetSocketTransform` (`self.StaticMeshComponent`) `Socket Name` "RTS_ParentBoneSpace")))
  (return _returnvalue_location))

(fn `ShootWeapon`
  (bind _returnvalue (`GameplayStatics.GetPlayerPawn` 0))
  (bind (_returnvalue_location _returnvalue_rotation) (`KismetMathLibrary.BreakTransform` (`SceneComponent.GetSocketTransform` (`self.StaticMeshComponent`) "Muzzle" "RTS_World")))
  (if (<= (`self.ShootGap`) 0.0)
    (bind _returnvalue_2 (`|SpawnActorFromClass` "/Game/My/Blueprint/Character/Girl/Weapon/BP_MyMatchGun.BP_MyMatchGun_C" (`KismetMathLibrary.MakeTransform` _returnvalue_location _returnvalue_rotation) "Undefined" "OverrideRootScale" _returnvalue _returnvalue))
    (`MatchGun.FireInDirection` _returnvalue_2 (`KismetMathLibrary.Conv_RotatorToVector` _returnvalue_rotation))
    (set `self.ShootGap` (`self.TimeGap`))))

(fn `UserConstructionScript`)