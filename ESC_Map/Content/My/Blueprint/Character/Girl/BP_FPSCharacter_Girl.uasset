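; First-person girl character Blueprint that fires a weapon held as a child actor.
; TriggerRight press and release both feed one FlipFlop that toggles the Shoot flag, so holding the trigger means firing.
; While Shoot is set, Tick casts the child actor to BP_GirlWeapon and calls ShootWeapon every frame.
; GetSocketPosition forwards socket position queries to that same weapon.
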(event `self.ReceiveBeginPlay`)

(event `self.ReceiveTick`
  (params (DeltaSeconds :type "Float (single-precision)"))
  (if (`self.Shoot`)
    (bind _asbp_girl_weapon (cast `/Game/My/Blueprint/Character/Girl/Weapon/BP_GirlWeapon` (`ChildActorComponent.ChildActor` (`self.BP_GirlWeapon`))))
    (`/Game/My/Blueprint/Character/Girl/Weapon/BP_GirlWeapon.ShootWeapon` _asbp_girl_weapon)))

(event `InputAction|TriggerRight`
  (params (Key :type "Key Structure"))
  (:`Pressed`
    (bind _isa (`/Engine/EditorBlueprintResources/StandardMacros.FlipFlop` :!label _label)
      (:`A`
        _)
      (:`B`
        _))
    (set `self.Shoot` _isa))
  (:`Released`
    (goto _label)))

(fn `Get Socket Position`
  (params (`Socket Name` :type Name))
  (returns (Position :type "Vector Structure"))
  (bind _asbp_girl_weapon (cast `/Game/My/Blueprint/Character/Girl/Weapon/BP_GirlWeapon` (`ChildActorComponent.ChildActor` (`self.BP_GirlWeapon`))))
  (bind _socket_position (`/Game/My/Blueprint/Character/Girl/Weapon/BP_GirlWeapon.Get Scoekt Position` _asbp_girl_weapon `Socket Name`))
  (return _socket_position))

(fn `UserConstructionScript`)