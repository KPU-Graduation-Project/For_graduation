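; BP_Girl_MotionControl is a VR girl character blueprint that fires its weapon from the right trigger.
; On BeginPlay it sets an eye-level tracking origin and moves the capsule to the CameraHeight offset.
; Trigger press and release share one FlipFlop that toggles Shoot, and Tick calls ShootWeapon on GirlWeapon every frame while Shoot is true.
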(event `self.ReceiveBeginPlay`
  (`HeadMountedDisplayFunctionLibrary.SetTrackingOrigin` "Eye")
  (`SceneComponent.K2_SetRelativeLocation` (`self.CapsuleComponent`) (`self.Camera Height`) false false))

(event `self.ReceiveTick`
  (params (DeltaSeconds :type "Float (single-precision)"))
  (if (`self.Shoot`)
    (`/Game/My/Blueprint/Character/Girl/Girl_Weapon_Component.Shoot Weapon` (`self.Girl Weapon`))))

(event `InputAction|TriggerRight`
  (params (Key :type "Key Structure"))
  (:`Pressed`
    (bind _isa (`/Engine/EditorBlueprintResources/StandardMacros.FlipFlop` :!label _label)
      (:`A`
        _)
      (:`B`
        _))
    (set `self.Shoot` _isa))
  (:`Released`
    (goto _label)))

(fn `UserConstructionScript`)